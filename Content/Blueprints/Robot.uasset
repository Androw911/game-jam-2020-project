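; Player-controllable 2D flipbook Robot that flies in the YZ plane, hits or repairs other robots, and carries Krabica boxes.
; Axis input feeds Tick movement, while action animations play to their last frame and key 0 possesses another Robot.
; Repairs raise SpeedUpgrade and non-Robot collisions lower it, scaling speed and toggling spark and lightning effects.
; Hits knock robots back and detach boxes, and Tick derives X from height, apparently for depth sorting.
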(event `Key|Zero`
  (params (Key :type "Key Structure"))
  (bind _returnvalue (`GameplayStatics.GetPlayerControllerFromID` 0))
  (:`Pressed`
    (bind _outactors (`GameplayStatics.GetAllActorsOfClass` "Robot_C"))
    (for _array_element _outactors
      (if (!= _returnvalue (`self.GetInstigatorController` (`ActorComponent.GetOwner` (`Actor.RootComponent` _array_element))))
        (`Controller.Possess` _returnvalue _array_element)
        (break)))))

(event `InputAxis|Z_Axis`
  (params (AxisValue :type "Float (single-precision)"))
  ;[1 1 1] Movement
  (set `self.Current up speed` (* (* 30000 AxisValue) (`GameplayStatics.GetWorldDeltaSeconds`)))
  (bind _isanimationinprogress (`self.Update animations` (!= (stale `InputAxis|X_Axis` AxisValue) 0.0) (!= AxisValue 0.0)))
  (bind _output_get (set `self.isAnimationInProgress` _isanimationinprogress))
  (if (`self.isPickingUp`)
    (set `self.isPickingUp` _output_get)))

(event `InputAxis|X_Axis`
  (params (AxisValue :type "Float (single-precision)"))
  (bind _returnvalue (!= AxisValue 0.0))
  ;[1 1 1] Movement
  (set `self.Current forward speed` (* (* -30000 AxisValue) (`GameplayStatics.GetWorldDeltaSeconds`)))
  (bind _isanimationinprogress (`self.Update animations` _returnvalue (!= (stale `InputAxis|Z_Axis` AxisValue) 0.0)))
  (set `self.isAnimationInProgress` _isanimationinprogress)
  (if _returnvalue
    (`self.Rotate actor` (`self.GetInputAxisValue`))))

(event `InputAction|Hit_Action`
  (params (Key :type "Key Structure"))
  ;[1 1 1] Hit Action
  (:`Pressed`
    (if (and (not (`self.isCarryingBox`)) (not (`self.isAnimationInProgress`)))
      (`PaperFlipbookComponent.SetFlipbook` (`self.Sprite`) "/Game/flipbooks/anim-character-main-hit.anim-character-main-hit")
      (set `self.isAnimationInProgress` true)
      (for _array_element (`PrimitiveComponent.GetOverlappingActors` (`self.Capsule`) "Robot_C")
        (if (!= _array_element self)
          (`KismetSystemLibrary.PrintString` (`KismetSystemLibrary.GetDisplayName` _array_element))
          (bind _asrobot (cast `/Game/Blueprints/Robot` _array_element))
          (`self.Get hit` _asrobot self)
          (set `/Game/Blueprints/Robot.isAnimationInProgress` true _asrobot))))))

(event `InputAction|Repair_Action`
  (params (Key :type "Key Structure"))
  ;[1 1 1] Repair Action
  (:`Pressed`
    (if (and (not (`self.isCarryingBox`)) (not (`self.isAnimationInProgress`)))
      (`PaperFlipbookComponent.SetFlipbook` (`self.Sprite`) "/Game/flipbooks/anim-character-main-repair.anim-character-main-repair")
      (set `self.isAnimationInProgress` true)
      (for _array_element (`PrimitiveComponent.GetOverlappingActors` (`self.Capsule`) "Robot_C")
        (if (!= _array_element self)
          (`KismetSystemLibrary.PrintString` (`KismetSystemLibrary.GetDisplayName` _array_element))
          (bind _asrobot (cast `/Game/Blueprints/Robot` _array_element))
          (`self.Get repaired` _asrobot)
          (set `/Game/Blueprints/Robot.isAnimationInProgress` true _asrobot))))))

(event `InputAction|Pickup_Action`
  (params (Key :type "Key Structure"))
  (bind _charactermovement (`self.CharacterMovement`))
  (:`Pressed`
    (set `CharacterMovementComponent.MaxFlySpeed` 0.1 _charactermovement)
    (set `CharacterMovementComponent.MaxAcceleration` 0.0 _charactermovement)
    (set `self.isPickingUp` true)
    (set `self.isAnimationInProgress` true)
    (if (`self.isCarryingBox`)
      (`PaperFlipbookComponent.SetFlipbook` (`self.Sprite`) "/Game/flipbooks/anim-character-pick-up.anim-character-pick-up")
      (`self.K2_DetachFromActor` (`self.Carried box`) "KeepWorld" "KeepRelative" "KeepRelative")
      (`/Game/Blueprints/Krabica.setLastPlayerHolding` (`self.Carried box`) self)
      (`self.K2_SetActorTransform` (`self.Carried box`) (`KismetMathLibrary.MakeTransform` (`KismetMathLibrary.MakeVector` (.x (`SceneComponent.K2_GetComponentLocation` (`self.Capsule`))) (.y (`SceneComponent.K2_GetComponentLocation` (`self.Capsule`))) (- (.z (`SceneComponent.K2_GetComponentLocation` (`self.Capsule`))) 70.0))) false false)
      (set `self.isCarryingBox` false)
      (`/Game/Blueprints/Krabica.setIsBeingCarried` (`self.Carried box`) false)
      (else
        (`PaperFlipbookComponent.SetFlipbook` (`self.Sprite`) "/Game/flipbooks/anim-character-pick-up.anim-character-pick-up")
        (for _array_element (`PrimitiveComponent.GetOverlappingActors` (`self.Capsule`) "/Game/Blueprints/Krabica.Krabica_C")
          (bind _askrabica (cast `/Game/Blueprints/Krabica` _array_element))
          (if (and (== _array_element "/Game/Blueprints/Krabica.Krabica") (!= (`self.GetAttachParentActor` _askrabica) "Robot"))
            (break)))
        (bind _askrabica_2 (cast `/Game/Blueprints/Krabica` _array_element))
        (bind _output_get (set `self.Carried box` _askrabica_2))
        (`KismetSystemLibrary.Delay` 0.3)
        (`self.K2_AttachToActor` _output_get self "None" "KeepWorld" "KeepRelative" "KeepRelative" true)
        (`self.K2_SetActorTransform` (`self.Carried box`) (`KismetMathLibrary.MakeTransform` (`KismetMathLibrary.MakeVector` (.x (`SceneComponent.K2_GetComponentLocation` (`self.Capsule`))) (- (.y (`SceneComponent.K2_GetComponentLocation` (`self.Capsule`))) (select `bool` (== (.yaw (`self.GetControlRotation`)) 0.0) :`false` 20.0 :`true` -20.0 :!type "Float (single-precision)")) (- (.z (`SceneComponent.K2_GetComponentLocation` (`self.Capsule`))) 20.0))) false false)
        (bind _output_get_2 (set `self.isCarryingBox` true))
        (`/Game/Blueprints/Krabica.setIsBeingCarried` (`self.Carried box`) _output_get_2)))))

(event `self.ReceiveHit`
  (params (MyComp :type "PrimitiveComponent Object Reference") (Other :type "Actor Object Reference") (OtherComp :type "PrimitiveComponent Object Reference") (bSelfMoved :type Boolean) (HitLocation :type "Vector Structure") (HitNormal :type "Vector Structure") (NormalImpulse :type "Vector Structure") (Hit :type "HitResult Structure (by ref)"))
  (if (not (== (`GameplayStatics.GetObjectClass` Other) "Robot_C"))
    (`self.get damage`)
    (`PaperFlipbookComponent.SetFlipbook` (`self.Parts`) "/Game/flipbooks/anim-effect-parts.anim-effect-parts"))
  (`CharacterMovementComponent.AddImpulse` (`self.CharacterMovement`) (* HitNormal (* (`self.SpeedUpgrade`) (* 15 (`self.base speed`)))) false))

(event `self.ReceiveTick`
  (params (DeltaSeconds :type "Float (single-precision)"))
  (bind _bump_vector (`self.Bump vector`))
  (bind _speedupgrade (`self.SpeedUpgrade`))
  (bind _charactermovement (`self.CharacterMovement`))
  (bind _delta_seconds (`self.delta seconds`))
  (bind _base_speed (`self.base speed`))
  (bind _parts (`self.Parts`))
  (bind _z (.z (`SceneComponent.K2_GetComponentLocation` (`self.CapsuleComponent`))))
  (set `self.delta seconds` DeltaSeconds)
  (if (not (`self.isPickingUp`))
    (set `CharacterMovementComponent.MaxFlySpeed` (* _speedupgrade _base_speed) _charactermovement)
    (set `CharacterMovementComponent.MaxAcceleration` (* _speedupgrade _base_speed) _charactermovement)
    (`CharacterMovementComponent.SetMovementMode` (`self.CharacterMovement`) "MOVE_Flying" 0)
    (`self.AddMovementInput` (select `bool` (`AIBlueprintHelperLibrary.IsValidAIDirection` _bump_vector) :`false` (`KismetMathLibrary.MakeVector` 0.0 (* _delta_seconds (`self.Current forward speed`)) (* _delta_seconds (`self.Current up speed`))) :`true` (* _bump_vector _delta_seconds)))
    (`self.K2_SetActorLocation` (`KismetMathLibrary.MakeVector` (/ _z -100.0) (.y (`SceneComponent.K2_GetComponentLocation` (`self.CapsuleComponent`))) _z))
    (`|ExecutionSequence`
      (:`then_0`
        (if (`AIBlueprintHelperLibrary.IsValidAIDirection` (`self.Bump vector`))
          (set `self.Bump vector` (0.0 0.0 0.0))))
      (:`then_1`
        (bind _isfinished (`self.Finish previous animation` _parts))
        (if _isfinished
          (`PaperFlipbookComponent.SetFlipbook` _parts null))))))

(fn `Finish previous animation`
  (params (`target flipbook` :type "PaperFlipbookComponent Object Reference"))
  (returns (isFinished :type Boolean))
  (return (not (!= (`PaperFlipbookComponent.GetPlaybackPositionInFrames` `target flipbook`) (- (`PaperFlipbookComponent.GetFlipbookLengthInFrames` `target flipbook`) 1)))))

(fn `get damage`
  (if (> (`self.SpeedUpgrade`) 1)
    (bind _result (`/Engine/EditorBlueprintResources/StandardMacros.DecrementInt` (`self.SpeedUpgrade`))
      (:`  `
        (if (< _result 4)
          (`PaperFlipbookComponent.SetFlipbook` (select `int` 0 :`0` (`self.Sparks`) :`1` (`self.Sparks1`) :`2` (`self.Sparks2`)) "/Game/flipbooks/anim-effect-sparks.anim-effect-sparks")
          (if (< (`self.SpeedUpgrade`) 8)
            (`PaperFlipbookComponent.SetFlipbook` (select `int` 0 :`0` (`self.Lighting`) :`1` (`self.Lighting1`) :`2` (`self.Lighting2`) :`3` (`self.Lighting3`)) "/Game/flipbooks/anim-effect-lightning.anim-effect-lightning")))))))

(fn `Get hit`
  (params (Attacker :type "/Game/Blueprints/Robot Object Reference"))
  (locals (NewLocalVar_0 :type "/Game/Blueprints/Robot Object Reference"))
  (`PaperFlipbookComponent.SetFlipbook` (`self.Sprite`) "/Game/flipbooks/anim-character-main-got-hit.anim-character-main-got-hit")
  (`Controller.SetControlRotation` (`self.GetController`) (select `bool` (== (.yaw (`self.GetControlRotation` Attacker)) 0.0) :`false` (`KismetMathLibrary.MakeRotator` 0.0) :`true` (`KismetMathLibrary.MakeRotator` 0.0 0.0 180.0)))
  (if (`KismetSystemLibrary.IsValid` (`self.Carried box`))
    (`self.K2_DetachFromActor` (`self.Carried box`) "KeepWorld" "KeepRelative" "KeepRelative")
    (set `self.isCarryingBox` false))
  (`CharacterMovementComponent.AddImpulse` (`self.CharacterMovement`) (* (`SceneComponent.GetForwardVector` (`/Game/Blueprints/Robot.Arrow1` (`local.Attacker`))) 80000) false))

(fn `Get repaired`
  (bind _speedupgrade (`self.SpeedUpgrade`))
  (`PaperFlipbookComponent.SetFlipbook` (`self.Sprite`) "/Game/flipbooks/anim-character-main-got-repaired.anim-character-main-got-repaired")
  (if (< _speedupgrade 8)
    (`/Engine/EditorBlueprintResources/StandardMacros.IncrementInt` (`self.SpeedUpgrade`)
      (:`  `
        (`PaperFlipbookComponent.SetFlipbook` (select `int` (- _speedupgrade 1) :`0` (`self.Lighting3`) :`1` (`self.Lighting2`) :`2` (`self.Lighting1`) :`3` (`self.Lighting`) :`4` (`self.Sparks2`) :`5` (`self.Sparks1`) :`6` (`self.Sparks`)) null)))))

(fn `Rotate actor`
  (params (axisValue :type "Float (double-precision)"))
  (`Controller.SetControlRotation` (`self.GetController`) (select `bool` (< axisValue 0.0) :`false` (`KismetMathLibrary.MakeRotator` 0.0 0.0 180.0) :`true` (`KismetMathLibrary.MakeRotator` 0.0))))

(fn `Update animations`
  (params (isMoving :type Boolean) (isMovingUp :type Boolean))
  (returns (isAnimationInProgress :type Boolean))
  (if (`self.isAnimationInProgress`)
    (bind _isfinished (`self.Finish previous animation` (`self.Sprite`)))
    (return (not _isfinished))
    (elif (not (`self.isCarryingBox`))
      (`PaperFlipbookComponent.SetFlipbook` (`self.Sprite`) (select `bool` (or isMoving isMovingUp) :`false` "/Game/flipbooks/anim-character-main-idle.anim-character-main-idle" :`true` "/Game/flipbooks/anim-character-main-move.anim-character-main-move" :!type "PaperFlipbook Object Reference"))
      (return false)
      (else
        (`PaperFlipbookComponent.SetFlipbook` (`self.Sprite`) "/Game/flipbooks/anim-character-carry.anim-character-carry")
        (return false)))))

(fn `UserConstructionScript`)