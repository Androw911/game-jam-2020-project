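; Battlefield map Blueprint that lays out a 14x7 obstacle grid with a hard-coded set of platforms and props.
; Init sizes and clears the flat row-major grid, then places each obstacle via AddObstacle.
; ObstacleFactory maps a type index to footprint, sprite or flipbook, passability and an Accepts value.
; AddObstacle records position and type in ObstacleList and writes the footprint's cells through SetCell.
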(event `self.ReceiveBeginPlay`)

(fn `addObstacle`
  (params (Index :type Integer) (x :type Integer) (y :type Integer))
  (bind _obstaclelist (`self.obstacleList`))
  (bind (_width _height) (`self.Obstacle Factory` Index))
  (`KismetArrayLibrary.Array_Insert` _obstaclelist (make `IntVector` x y Index) (`KismetArrayLibrary.Array_Length` _obstaclelist))
  (for _index (range y (+ _height y))
    (for _index_2 (range x (+ _width x))
      (`self.setCell` _index_2 _index Index))))

(fn `getCell`
  (params (x :type Integer) (y :type Integer))
  (returns (`Cell type` :type Integer))
  (return (`|GetArrayItem` (`self.obstacleGrid`) (+ x (* y (`self.width`))))))

(fn `init`
  (set `self.width` 14)
  (set `self.height` 7)
  (`self.initGrid`)
  (`self.addObstacle` 6)
  (`self.addObstacle` 2 5)
  (`self.addObstacle` 2 10)
  (`self.addObstacle` 3 0 4)
  (`self.addObstacle` 4 5 4)
  (`self.addObstacle` 5 10 4))

(fn `initGrid`
  (returns (created :type Boolean))
  (bind _width (`self.width`))
  (for _index (range (`self.height`))
    (for _index_2 (range _width)
      (`KismetArrayLibrary.Array_Set` (`self.obstacleGrid`) (+ _index_2 (* _width _index)) 0 true)))
  (return true))

(fn `Obstacle Factory`
  (params (index :type Integer))
  (returns (width :type Integer) (height :type Integer) (sprite :type "PaperFlipbook Object Reference") (passable :type Boolean) (accepts :type Integer))
  (switch `int` index
    (:`0`
      (return 1 1 "/Game/flipbooks/platform1.platform1" true 0) ; podavac 1
    )
    (:`1`
      (return 1 1 "/Game/flipbooks/platform2.platform2" true 1) ; podavac 2
    )
    (:`2`
      (return 1 1 "/Game/flipbooks/platform3.platform3" true 2) ; podavac 3
    )
    (:`3`
      (return 1 2 "/Game/flipbooks/gizmo-1x.gizmo-1x" false -1) ; Gizmo A
    )
    (:`4`
      (return 2 2 "/Game/flipbooks/gizmo-2x.gizmo-2x" false -1) ; Gizmo B
    )
    (:`5`
      (return 1 1 "/Game/flipbooks/barrel_Flipbook.barrel_Flipbook" false -1) ; Barrel
    )
    (:`6`
      (return 3 1 "/Game/flipbooks/fence_Flipbook.fence_Flipbook" false -1) ; Plot
    )))

(fn `setCell`
  (params (x :type Integer) (y :type Integer) (`Cell type` :type Integer))
  (`KismetArrayLibrary.Array_Set` (`self.obstacleGrid`) (+ x (* y (`self.width`))) `Cell type`))