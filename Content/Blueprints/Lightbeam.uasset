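; Lightbeam Blueprint that scatters child actor components, apparently sparks, inside the bounds of its Sparks box.
; SpawnSparks adds one component at a random point in that box and prints a debug "Hello".
; It runs from the construction script, BeginPlay and every Tick, so components are added each frame with no removal shown.
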(event `self.ReceiveBeginPlay`
  (`self.SpawnSparks`))

(event `self.ReceiveTick`
  (params (DeltaSeconds :type "Float (single-precision)"))
  (`self.SpawnSparks`))

(fn `SpawnSparks`
  (returns (ReturnValue :type "/Game/Blueprints/dust-particle Object Reference"))
  (bind _sparks (`self.sparks`))
  (`AddComponent|NODE_AddChildActorComponent-2` :`RelativeTransform` (`KismetMathLibrary.Conv_VectorToTransform` (`KismetMathLibrary.RandomPointInBoundingBox` (`SceneComponent.RelativeLocation` _sparks) (`BoxComponent.BoxExtent` _sparks))))
  (`KismetSystemLibrary.PrintString` "Hello")
  (return null))

(fn `UserConstructionScript`
  (`self.SpawnSparks`))