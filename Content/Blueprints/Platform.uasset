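; Platform is a typed 2D actor that checks whether an overlapping Krabica matches its type, apparently as a target in a matching puzzle.
; SetType stores the type and swaps the Paper2D flipbook among three Krabica visuals, defaulting to the first.
; IsEngaged queries the Box for overlapping Krabica actors, prints both types for debugging, and returns the comparison for the first one found only.
; Event graph and construction script are empty.
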(fn `isEngaged`
  (returns (engaged :type Boolean))
  (bind _type (`self.Type`))
  (for _array_element (`PrimitiveComponent.GetOverlappingActors` (`self.Box`) "/Game/Blueprints/Krabica.Krabica_C")
    (bind _askrabica (cast `/Game/Blueprints/Krabica` _array_element))
    (bind _type_2 (`/Game/Blueprints/Krabica.Type` _askrabica))
    (`KismetSystemLibrary.PrintString` (`KismetStringLibrary.Concat_StrStr` "platform: " (`KismetStringLibrary.Conv_IntToString` _type) ", krabica: " (`KismetStringLibrary.Conv_IntToString` _type_2)))
    (return (== _type _type_2))))

(fn `Set Type`
  (params (type :type Integer))
  (bind _paperflipbook (`self.PaperFlipbook`))
  (bind _output_get (set `self.Type` type))
  (switch `int` _output_get
    (:`Default`
      (`PaperFlipbookComponent.SetFlipbook` _paperflipbook "/Game/flipbooks/krabica1.krabica1" :!label _label))
    (:`0`
      (goto _label))
    (:`1`
      (`PaperFlipbookComponent.SetFlipbook` _paperflipbook "/Game/flipbooks/krabica2.krabica2"))
    (:`2`
      (`PaperFlipbookComponent.SetFlipbook` _paperflipbook "/Game/flipbooks/krabica3.krabica3"))))

(fn `UserConstructionScript`)