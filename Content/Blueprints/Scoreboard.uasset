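; Scoreboard Blueprint that shows a two-digit score using Paper2D flipbook digits.
; SetScore splits the score into units (modulo 10) and tens (integer division by 10), passing each to SetUnit and SetDecimal.
; Each setter switches on the digit 0–9 and assigns the matching numeral flipbook to the Unit or Decimal component.
; The event graph and construction script are empty, so updates rely on SetScore being called.
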(event `self.ReceiveBeginPlay`)

(fn `setDecimal`
  (params (decimal :type Integer))
  (bind _decimal (`self.decimal`))
  (switch `int` decimal
    (:`0`
      (`PaperFlipbookComponent.SetFlipbook` _decimal "/Game/flipbooks/0.0"))
    (:`1`
      (`PaperFlipbookComponent.SetFlipbook` _decimal "/Game/flipbooks/1.1"))
    (:`2`
      (`PaperFlipbookComponent.SetFlipbook` _decimal "/Game/flipbooks/2.2"))
    (:`3`
      (`PaperFlipbookComponent.SetFlipbook` _decimal "/Game/flipbooks/3.3"))
    (:`4`
      (`PaperFlipbookComponent.SetFlipbook` _decimal "/Game/flipbooks/4.4"))
    (:`5`
      (`PaperFlipbookComponent.SetFlipbook` _decimal "/Game/flipbooks/5.5"))
    (:`6`
      (`PaperFlipbookComponent.SetFlipbook` _decimal "/Game/flipbooks/6.6"))
    (:`7`
      (`PaperFlipbookComponent.SetFlipbook` _decimal "/Game/flipbooks/7.7"))
    (:`8`
      (`PaperFlipbookComponent.SetFlipbook` _decimal "/Game/flipbooks/8.8"))
    (:`9`
      (`PaperFlipbookComponent.SetFlipbook` _decimal "/Game/flipbooks/9.9"))))

(fn `setScore`
  (params (score :type Integer))
  (`self.setUnit` (mod score 10))
  (`self.setDecimal` (/ score 10)))

(fn `setUnit`
  (params (decimal :type Integer))
  (bind _unit (`self.unit`))
  (switch `int` decimal
    (:`0`
      (`PaperFlipbookComponent.SetFlipbook` _unit "/Game/flipbooks/0.0"))
    (:`1`
      (`PaperFlipbookComponent.SetFlipbook` _unit "/Game/flipbooks/1.1"))
    (:`2`
      (`PaperFlipbookComponent.SetFlipbook` _unit "/Game/flipbooks/2.2"))
    (:`3`
      (`PaperFlipbookComponent.SetFlipbook` _unit "/Game/flipbooks/3.3"))
    (:`4`
      (`PaperFlipbookComponent.SetFlipbook` _unit "/Game/flipbooks/4.4"))
    (:`5`
      (`PaperFlipbookComponent.SetFlipbook` _unit "/Game/flipbooks/5.5"))
    (:`6`
      (`PaperFlipbookComponent.SetFlipbook` _unit "/Game/flipbooks/6.6"))
    (:`7`
      (`PaperFlipbookComponent.SetFlipbook` _unit "/Game/flipbooks/7.7"))
    (:`8`
      (`PaperFlipbookComponent.SetFlipbook` _unit "/Game/flipbooks/8.8"))
    (:`9`
      (`PaperFlipbookComponent.SetFlipbook` _unit "/Game/flipbooks/9.9"))))

(fn `UserConstructionScript`)