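; Multiplayer Blueprint that sets match defaults and spawns local players as Robots when play begins.
; SetDefaults fills tuning variables for boxes, obstacles, movement, health, score and time limits, and damage and repair with cooldowns.
; CreatePlayers then creates one local player per PlayerStart, using the array index as controller ID and falling back to the existing controller if creation fails.
; Each controller possesses a Robot spawned at that start's transform.
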(event `self.ReceiveBeginPlay`
  (`self.setDefaults`)
  (`self.CreatePlayers`))

(fn `CreatePlayers`
  (bind _outactors (`GameplayStatics.GetAllActorsOfClass` "/Script/Engine.PlayerStart"))
  (for (_array_element _array_index) _outactors
    (bind _returnvalue (`GameplayStatics.CreatePlayer` _array_index))
    (bind _output_get (set `self.Player` _returnvalue))
    (if (not (`KismetSystemLibrary.IsValid` _output_get))
      (bind _output_get_2 (set `self.Player` (`GameplayStatics.GetPlayerControllerFromID` _array_index))))
    (bind _returnvalue_2 (`|SpawnActorFromClass` "/Game/Blueprints/Robot.Robot_C" (`self.GetTransform` _array_element) "Undefined" "OverrideRootScale" _output_get_2 null))
    (`Controller.Possess` (`self.Player`) _returnvalue_2)))

(fn `setDefaults`
  (set `self.boxTypeCount` 3)
  (set `self.obstacleDensity` 2)
  (set `self.maxSpeed` 1.0)
  (set `self.minHealth` 0.1)
  (set `self.maxHealth` 0.9)
  (set `self.dampening` 1.0)
  (set `self.scoreLimit` 10)
  (set `self.timeLimit` 300)
  (set `self.damageValue` 0.1)
  (set `self.damageCooldown` 1.0)
  (set `self.repairValue` 0.1)
  (set `self.repairCooldown` 1.0))

(fn `UserConstructionScript`)